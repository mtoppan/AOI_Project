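; BP_AudioControl starts its Audio component on BeginPlay and calls SpawnGrid, apparently an unfinished setup for an audio-driven grid of cubes.
; SpawnGrid loops over NumberOfCubes with an empty body, so it spawns nothing.
; Disconnected nodes sketch a square layout from row, column and Distance, wrapping rows at the square root of the count.
; The Synesthesia cube function is an empty stub.
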(event EventBeginPlay
  (Audio|Components|Audio|Play (Variables|Default|GetAudio) 0.0)
  (CallFunction|SpawnGrid))

(event Collision|EventActorBeginOverlap
  (params (OtherActor :type Actor%20Object%20Reference)))

(event EventTick
  (params (DeltaSeconds :type Float%20%28single-precision%29)))

(fn ConstructionScript)

(fn SpawnGrid
  (for _index (range 0 (- (Variables|Default|GetNumber%20of%20Cubes) 1))
    _))

(fn SynesthesiaCube
  (params (NewParam :type Float%20%28double-precision%29)))