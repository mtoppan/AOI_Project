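; BP_Ball is an actor that animates its Rock component as a bouncing ball, timed to a BPM value.
; On BeginPlay it sets the timeline play rate relative to 120 BPM and plays it.
; Timeline tracks drive the Rock's vertical and sideways (local Y) offsets plus a squash in scale.
; A Hit Ground event track spawns a particle effect at the Rock's location.
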(event EventBeginPlay
  (bind _rock (Variables|Default|GetRock))
  (Components|Timeline|SetPlayRate (Variables|Default|GetTimeline_Rock) (/ (Variables|Default|GetBPM) 1.2e+02))
  (bind (_direction _z_movement _size _x_movement) (Timeline|Timeline_Rock Play)
    (:Update
      (Transformation|SetRelativeLocation _rock (+ (Math|Vector|Lerp(Vector) "0, 0, 0" "0.000000,0.000000,500.000000" _z_movement) (Math|Vector|Lerp(Vector) "0, 0, 0" "0.000000,1000.000000,0.000000" _x_movement)) false false)
      (Transformation|SetRelativeScale3D _rock (Math|Vector|Lerp(Vector) "0.500000,0.500000,0.500000" "0.550000,0.550000,0.450000" _size)))
    (:HitGround
      (Effects|SpawnEmitteratLocation "/Engine/Tutorial/SubEditors/TutorialAssets/TutorialParticleSystem.TutorialParticleSystem" (Transformation|GetWorldLocation _rock)))))

(fn ConstructionScript)