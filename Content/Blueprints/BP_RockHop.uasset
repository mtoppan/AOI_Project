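; BP_RockHop is a rock actor that plays landing effects and fades its materials in response to a playing percussion instrument.
; BeginPlay hides the boulder geometry collection and creates two dynamic materials, whose Alpha a timeline animates when an overlapping "Instrument"-tagged PercussionInstrument is playing.
; PlayLandSFX plays an attenuated bounce sound and briefly pulses Niagara dust.
; The overlap check does not yet single out drums.
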(event Custom|PlayLandSFX
  (Audio|PlaySoundatLocation "/Game/Sounds/SFX/rockBounceLarge.rockBounceLarge" (Transformation|GetActorLocation) "0, 0, 0" 1.0 1.0 0.0 "/Game/Sounds/SFX/SA_Rocks.SA_Rocks" 0 0 0)
  (Components|Activation|Activate (Variables|Default|GetNS_Dust) false)
  (Utilities|FlowControl|Delay 0.2)
  (Components|Activation|Deactivate (Variables|Default|GetNS_Dust)))

(event Custom|FadeAlpha
  (bind _alphatrack (Timeline|ChangeAlpha Play)
    (:Update
      (Rendering|Material|SetScalarParameterValue (stale EventBeginPlay _returnvalue) "Alpha" _alphatrack :!class /Script/Engine.MaterialInstanceDynamic)
      (Rendering|Material|SetScalarParameterValue (stale EventBeginPlay _returnvalue_2) "Alpha" _alphatrack :!class /Script/Engine.MaterialInstanceDynamic))))

(event Collision|EventActorBeginOverlap
  (params (OtherActor :type Actor%20Object%20Reference))
  (if (Actor|ActorHasTag OtherActor "Instrument")
    (bind _aspercussion_instrument (Utilities|Casting|CastToPercussionInstrument OtherActor))
    (if (Variables|/Script/AOI_Project.PercussionInstrument|GetPlaying _aspercussion_instrument)
      (CallFunction|FadeAlpha))))

(event EventBeginPlay
  (Rendering|SetVisibility (Variables|Default|Getboulder_hop_GeometryCollection) false false)
  (bind _returnvalue (Rendering|Material|CreateDynamicMaterialInstance (Variables|Default|Getboulder_hop_GeometryCollection) 0 0 "None" :!class /Script/Engine.PrimitiveComponent))
  (bind _returnvalue_2 (Rendering|Material|CreateDynamicMaterialInstance (Variables|Default|Getboulder_hop_GeometryCollection) 1 0 "None" :!class /Script/Engine.PrimitiveComponent)))

(fn ConstructionScript)