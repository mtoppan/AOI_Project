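; BP_Spawn is a spawner actor that drops a short burst of BP_Ball actors when triggered.
; Its Ball function sets the RockStart flag, which Tick polls and clears as it spawns, so each trigger gives one burst.
; A small loop places each ball at a random XY point within a fixed area at zero height, always spawning despite collisions, with a short lifespan for automatic cleanup.
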(event EventTick
  (params (DeltaSeconds :type Float%20%28single-precision%29))
  (if (Variables|Default|GetRockStart)
    (for _index (range 0 3)
      (bind _output_get (Variables|Default|Setposition (Math|Vector|MakeVector (Math|Random|RandomFloatinRange -1e+03 -2e+02) (Math|Random|RandomFloatinRange 3.6e+03 4.4e+03) 0.0)))
      (bind _returnvalue (Game|SpawnActorfromClass "/Game/BP_Ball.BP_Ball_C" (Math|Conversions|ToTransform(Vector) _output_get) "AdjustIfPossibleButAlwaysSpawn" 0 0))
      (Actor|SetLifeSpan _returnvalue 2.4)
      (Variables|Default|SetRockStart false))))

(fn ConstructionScript)

(fn Ball
  (params (isTrigger :type Boolean))
  (Variables|Default|SetRockStart isTrigger))