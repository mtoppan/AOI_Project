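; BP_Flower is a one-time flower trigger that opens when the player touches it and counts toward the progress of BP_Gate.
; First overlap plays the open animation through the daisy AnimBlueprint, swaps the aura for a shrink effect and updates linked trees' animations.
; ShowParticlePath, not called within this graph, fires an opening burst and a timeline that moves a Niagara system along a spline, then notifies the gate.
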(event Custom|FlowerParticle
  (Components|Activation|Activate (Variables|Default|GetNS_Flower_System) false)
  (Components|Timeline|SetPlayRate (Variables|Default|GetMover) (/ 1.0 (Variables|Default|GetDuration)))
  (Components|Timeline|SetNewTime (Variables|Default|GetMover) (Variables|Default|GetStartOffset))
  (bind _alpha (Timeline|Mover Play)
    (:Update
      (Variables|Default|Setalpha _alpha)
      (Transformation|SetWorldLocation (Variables|Default|GetNS_Flower_System) (Spline|GetLocationatDistanceAlongSpline (Variables|Default|GetSpline) (Math|Float|Lerp 0.0 (Spline|GetSplineLength (Variables|Default|GetSpline)) (Variables|Default|Getalpha)) "World") false false))
    (:Finished
      (bind _returnvalue (Actor|GetActorOfClass "/Game/Blueprints/BP_Level2/BP_Gate.BP_Gate_C"))
      (Class|Gate|UpdateFlowersComplete _returnvalue)
      (Variables|Default|SetFinished true))))

(event Custom|FadeAwayNS
  (Components|Activation|Deactivate (Variables|Default|GetNS_FlowerAura))
  (Components|Activation|Activate (Variables|Default|GetNS_FlowerAuraShrink) false)
  (CallFunction|TurnOffTrees))

(event Custom|ShowParticlePath
  (Components|Activation|Activate (Variables|Default|GetNS_FlowerOpen) false)
  (CallFunction|FlowerParticle))

(event Custom|TurnOffTrees
  (for _array_element (Variables|Default|GetFlowersTrees)
    (Default|ChangeAnim _array_element false)))

(event EventBeginPlay
  (bind _asdaisy_animated_skeleton_anim_blueprint (Utilities|Casting|CastTodaisyAnimated_Skeleton_AnimBlueprint (Components|SkeletalMesh|GetAnimInstance (Variables|Default|GetdaisyAnimated))))
  (Variables|Default|SetFlowerAnim _asdaisy_animated_skeleton_anim_blueprint))

(event Collision|EventActorBeginOverlap
  (params (OtherActor :type Actor%20Object%20Reference))
  (if (Actor|ActorHasTag OtherActor "Player")
    (if (Variables|Default|GetFirstTime)
      (Variables|Default|SetFirstTime false)
      (Default|OpenFlower (Variables|Default|GetFlowerAnim))
      (CallFunction|FadeAwayNS))))

(fn ConstructionScript)