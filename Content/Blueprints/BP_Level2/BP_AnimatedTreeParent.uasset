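; BP_AnimatedTreeParent is a Level 2 parent Blueprint that switches animation on or off for up to three trees.
; Its ChangeAnim event passes the StartAnimation value to the Begin variable on each of three tree Anim Blueprint references, skipping any that are invalid.
; The references are not assigned in this graph, and the construction script is empty.
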(event Custom|ChangeAnim
  (params (StartAnimation? :type Boolean))
  (bind _tree1animbp (Variables|Default|GetTree1AnimBP))
  (bind _tree2animbp (Variables|Default|GetTree2AnimBP))
  (bind _tree3animbp (Variables|Default|GetTree3AnimBP))
  (if (Utilities|IsValid _tree1animbp)
    (Variables|/Game/Animations/Tree1_AnimBP.Tree1_AnimBP_C|SetBegin _tree1animbp StartAnimation?))
  (if (Utilities|IsValid _tree2animbp)
    (Variables|/Game/Animations/Tree2_AnimBP.Tree2_AnimBP_C|SetBegin _tree2animbp StartAnimation?))
  (if (Utilities|IsValid _tree3animbp)
    (Variables|/Game/Animations/Tree3_Anim3.Tree3_Anim3_C|SetBegin _tree3animbp StartAnimation?)))

(fn ConstructionScript)