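; BP_Gate is the Level 2 final gate that reacts to flower progress and reveals the final path.
; UpdateFlowerEffects plays an arrival effect, then cycles through three child BP_GateFlower actors to open one based on its Flower's FirstTime and Finished flags, looping back if none qualifies.
; Separate events play all-arrived effects and enable sphere overlaps, trigger gate animation and sound, and destroy the blocking box.
; The overlap-driven all-flowers check is disconnected.
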(event Custom|RemoveWall
  (Components|DestroyComponent (Variables|Default|GetBox)))

(event EventGateAnimationandEffects
  (Default|RevealFinalPath (Variables|Default|GetAnimBP))
  (Audio|PlaySoundatLocation "/Game/Sounds/SFX/gateOpenFINAL.gateOpenFINAL" (Transformation|GetActorLocation) "0, 0, 0" 1.0 1.0 0.0 0 0 0 0))

(event Collision|EventActorBeginOverlap
  (params (OtherActor :type Actor%20Object%20Reference)))

(event EventUpdateFlowerEffects
  (Audio|Components|Audio|Play (Variables|Default|GetParticleArrive) 0.0)
  (bind _asbp_gate_flower (Utilities|Casting|CastToBP_GateFlower (Variables|/Script/Engine.ChildActorComponent|GetChildActor (Variables|Default|GetBP_GateFlower)) :!label _label))
  (if (Variables|/Game/Blueprints/BP_Level2/BP_Flower.BP_Flower_C|GetFirstTime (Variables|/Game/Blueprints/BP_Level2/BP_GateFlower.BP_GateFlower_C|GetFlower _asbp_gate_flower)) ; first time false = opened
    (bind _asbp_gate_flower_2 (Utilities|Casting|CastToBP_GateFlower (Variables|/Script/Engine.ChildActorComponent|GetChildActor (Variables|Default|GetBP_GateFlower1)) :!label _label_2))
    (if (Variables|/Game/Blueprints/BP_Level2/BP_Flower.BP_Flower_C|GetFirstTime (Variables|/Game/Blueprints/BP_Level2/BP_GateFlower.BP_GateFlower_C|GetFlower _asbp_gate_flower_2))
      (bind _asbp_gate_flower_3 (Utilities|Casting|CastToBP_GateFlower (Variables|/Script/Engine.ChildActorComponent|GetChildActor (Variables|Default|GetBP_GateFlower2)) :!label _label_3))
      (if (Variables|/Game/Blueprints/BP_Level2/BP_Flower.BP_Flower_C|GetFirstTime (Variables|/Game/Blueprints/BP_Level2/BP_GateFlower.BP_GateFlower_C|GetFlower _asbp_gate_flower_3))
        (goto _label)
        (elif (Variables|/Game/Blueprints/BP_Level2/BP_Flower.BP_Flower_C|GetFinished (Variables|/Game/Blueprints/BP_Level2/BP_GateFlower.BP_GateFlower_C|GetFlower _asbp_gate_flower_3))
          (goto _label)
          (else
            (Default|OpenFlower _asbp_gate_flower_3))))
      (elif (Variables|/Game/Blueprints/BP_Level2/BP_Flower.BP_Flower_C|GetFinished (Variables|/Game/Blueprints/BP_Level2/BP_GateFlower.BP_GateFlower_C|GetFlower _asbp_gate_flower_2))
        (goto _label_3)
        (else
          (Default|OpenFlower _asbp_gate_flower_2))))
    (elif (Variables|/Game/Blueprints/BP_Level2/BP_Flower.BP_Flower_C|GetFinished (Variables|/Game/Blueprints/BP_Level2/BP_GateFlower.BP_GateFlower_C|GetFlower _asbp_gate_flower))
      (goto _label_2)
      (else
        (Default|OpenFlower _asbp_gate_flower)))))

(event EventFinalFlowerEffects
  (Audio|Components|Audio|Play (Variables|Default|GetAllParticlesArrive) 0.0)
  (Variables|/Script/Engine.PrimitiveComponent|SetbGenerateOverlapEvents (Variables|Default|GetSphere1) true))

(fn ConstructionScript)