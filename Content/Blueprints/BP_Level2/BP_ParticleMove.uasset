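; BP_ParticleMove is a level 2 actor that travels along a spline, apparently carrying a flower particle effect.
; The FlowerParticle event sets the Mover timeline's play rate from Duration and its start time from StartOffset, then plays it.
; Each update maps the timeline alpha to a distance along the TrackRef actor's spline and moves the actor to that world location.
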(event Custom|FlowerParticle
  (Development|PrintString "flower")
  (Components|Timeline|SetPlayRate (Variables|Default|GetMover) (/ 1.0 (Variables|Default|GetDuration)))
  (Components|Timeline|SetNewTime (Variables|Default|GetMover) (Variables|Default|GetStartOffset))
  (bind _alpha (Timeline|Mover Play)
    (:Update
      (Variables|Default|Setalpha _alpha)
      (Transformation|SetActorLocation (Spline|GetLocationatDistanceAlongSpline (Variables|/Game/Blueprints/BP_Level2/BP_Track.BP_Track_C|GetSpline (Variables|Default|GetTrackRef)) (Math|Float|Lerp 0.0 (Spline|GetSplineLength (Variables|/Game/Blueprints/BP_Level2/BP_Track.BP_Track_C|GetSpline (Variables|Default|GetTrackRef))) (Variables|Default|Getalpha)) "World") false false))))

(fn ConstructionScript)