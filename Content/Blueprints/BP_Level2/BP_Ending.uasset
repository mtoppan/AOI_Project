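; BP_Ending is a Level 2 ending actor that brings in the final UI and music.
; Its FinalMusicandUI event runs once behind a Done flag, fading in the FinalUI held by its widget component.
; An AddMusic timeline then drives the volume of the music manager's FinalAudio on each update.
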(event EventFinalMusicandUI
  (if (not (Variables|Default|GetDone))
    (bind _returnvalue (Actor|GetActorOfClass "/Game/Blueprints/BP_MusicManager.BP_MusicManager_C"))
    (bind _asfinal_ui (Utilities|Casting|CastToFinalUI (UserInterface|GetWidget (Variables|Default|GetWidget))))
    (Default|FadeinFin _asfinal_ui)
    (Variables|Default|SetDone true)
    (bind _volume (Timeline|AddMusic Play)
      (:Update
        (Audio|Components|Audio|AdjustVolume (Variables|/Game/Blueprints/BP_MusicManager.BP_MusicManager_C|GetFinalAudio _returnvalue) 0.0 _volume "Linear" :!class /Script/Engine.AudioComponent)))))

(fn ConstructionScript)