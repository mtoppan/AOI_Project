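; Level 2 gate flower that links itself to a matching BP_Flower and can play an opening animation.
; On BeginPlay, FlowerPosition selects one of three actor tags, and the tagged BP_Flower is cached in the Flower variable, which this graph does not otherwise use.
; The OpenFlower event sets the Open flag on its animation Blueprint, leaving the trigger to outside callers.
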(event Custom|OpenFlower
  (Variables|/Game/Animations/AnimBP_GateFlower.AnimBP_GateFlower_C|SetOpen (Variables|Default|GetAnimBP) true))

(event EventBeginPlay
  (if (== (Variables|Default|GetFlowerPosition) 0)
    (bind _outactors (Actor|GetAllActorswithTag "Flower0"))
    (for _array_element _outactors
      (bind _asbp_flower (Utilities|Casting|CastToBP_Flower _array_element))
      (Variables|Default|SetFlower _asbp_flower))
    (elif (== (Variables|Default|GetFlowerPosition) 1)
      (bind _outactors_2 (Actor|GetAllActorswithTag "Flower1"))
      (for _array_element_2 _outactors_2
        (bind _asbp_flower_2 (Utilities|Casting|CastToBP_Flower _array_element_2))
        (Variables|Default|SetFlower _asbp_flower_2))
      (elif (== (Variables|Default|GetFlowerPosition) 2)
        (bind _outactors_3 (Actor|GetAllActorswithTag "Flower2"))
        (for _array_element_3 _outactors_3
          (bind _asbp_flower_3 (Utilities|Casting|CastToBP_Flower _array_element_3))
          (Variables|Default|SetFlower _asbp_flower_3))))))

(fn ConstructionScript)