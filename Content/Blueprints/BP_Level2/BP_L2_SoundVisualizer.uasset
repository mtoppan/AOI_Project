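; Level 2 sound visualizer that makes its child crystal meshes glow blue with the loudness of an analyzed track.
; BeginPlay stores the sound's duration and creates dynamic M_crystal materials for the child primitive components.
; While BP_PercussionInstrument's drum track is on, Tick drives emissive and crystal colors from squared, pre-analyzed channel loudness.
; Playback position is estimated from looped game time with a fixed offset, not read from the audio.
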(event EventTick
  (params (DeltaSeconds :type Float%20%28single-precision%29))
  (bind _returnvalue (Utilities|Time|GetGameTimeinSeconds))
  (bind _duration (Variables|Default|GetDuration))
  (bind _analyzer (Variables|Default|GetAnalyzer))
  (bind _returnvalue_2 (- _returnvalue 0.160249))
  (bind _remainder (Class|KismetMathLibrary|FMod64 _returnvalue_2 _duration))
  (bind _outloudness (Class|LoudnessNRT|GetNormalizedChannelLoudnessatTime _analyzer _remainder 1))
  (bind _returnvalue_3 (* _outloudness _outloudness))
  (bind _returnvalue_4 (Math|Color|Lerp(LinearColor) "(R=0.000000,G=0.000000,B=0.000000,A=1.000000)" "(R=0.000000,G=0.027411,B=1.000000,A=1.000000)" _returnvalue_3))
  (for _array_element (Variables|Default|GetMatInstances)
    (bind _asmaterial_instance_dynamic (Utilities|Casting|CastToMaterialInstanceDynamic _array_element))
    (bind _returnvalue_5 (Actor|GetActorOfClass "/Game/Blueprints/BP_PercussionInstrument.BP_PercussionInstrument_C"))
    (if (Variables|/Game/Blueprints/BP_PercussionInstrument.BP_PercussionInstrument_C|GetDrumTrackOn _returnvalue_5)
      (Rendering|Material|SetVectorParameterValue _asmaterial_instance_dynamic "Emissive_Col" _returnvalue_4 :!class /Script/Engine.MaterialInstanceDynamic)
      (Rendering|Material|SetVectorParameterValue _asmaterial_instance_dynamic "Crystal_Col" _returnvalue_4 :!class /Script/Engine.MaterialInstanceDynamic))))

(event EventBeginPlay
  (bind _returnvalue (Actor|GetActorOfClass "/Game/Blueprints/BP_Level2/BP_soundTest.BP_soundTest_C"))
  (Variables|Default|SetAudio (Variables|/Game/Blueprints/BP_Level2/BP_soundTest.BP_soundTest_C|GetMeadowBrassWindsTrack _returnvalue))
  (Variables|Default|SetDuration (Variables|/Script/Engine.SoundBase|GetDuration (Variables|/Script/AudioAnalyzer.AudioAnalyzerNRT|GetSound (Variables|Default|GetAnalyzer))))
  (for _array_element (Components|GetChildrenComponents (Variables|Default|GetDefaultSceneRoot) false)
    (bind _asprimitive_component (Utilities|Casting|CastToPrimitiveComponent _array_element))
    (bind _returnvalue_2 (Rendering|Material|CreateDynamicMaterialInstance _asprimitive_component 0 "/Game/Materials/M_crystal.M_crystal" "None" :!class /Script/Engine.PrimitiveComponent))
    (Utilities|Array|Add (Variables|Default|GetMatInstances) _returnvalue_2)))

(fn ConstructionScript)