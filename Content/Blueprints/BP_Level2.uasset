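; BP_Level2 is an overlap trigger that handles the player's transition into level 2.
; When an actor tagged Player enters, it destroys the BP_SoundVisualizer (noted as the crystals) and clears GameLevel2 on BP_MusicManager.
; It moves the player's last checkpoint to its Respawn component and calls Level2UI on the HUD widget through a Gate.
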(event EventBeginPlay)

(event EventTick
  (params (DeltaSeconds :type Float%20%28single-precision%29)))

(event Collision|EventActorBeginOverlap
  (params (OtherActor :type Actor%20Object%20Reference))
  (if (Actor|ActorHasTag OtherActor "Player")
    (Development|PrintString "new level")
    ;[1 1 1] destroy crystals
    (bind _returnvalue (Actor|GetActorOfClass "/Game/Blueprints/BP_SoundVisualizer.BP_SoundVisualizer_C"))
    (Actor|DestroyActor _returnvalue)
    (bind _returnvalue_2 (Actor|GetActorOfClass "/Game/Blueprints/BP_MusicManager.BP_MusicManager_C"))
    (Variables|/Game/Blueprints/BP_MusicManager.BP_MusicManager_C|SetGameLevel2 _returnvalue_2 false) ; not respawn when dead
    (Development|PrintString (Utilities|String|ToString(Boolean) (Variables|/Game/Blueprints/BP_MusicManager.BP_MusicManager_C|GetGameLevel2 _returnvalue_2)))
    (bind _returnvalue_3 (Actor|GetActorOfClass "/Game/Blueprints/BP_Player.BP_Player_C"))
    (Variables|/Game/Blueprints/BP_Player.BP_Player_C|SetLastCheckpointLocation _returnvalue_3 (Transformation|GetWorldLocation (Variables|Default|Getrespawn)))
    (bind _asbp_hud (Utilities|Casting|CastToBP_HUD (HUD|GetHUD (Game|GetPlayerController 0))))
    (Utilities|FlowControl|Gate false
      (:Exit
        (Default|Level2UI (Variables|/Game/Blueprints/BP_HUD.BP_HUD_C|GetHUDWidget _asbp_hud))))))

(fn ConstructionScript)