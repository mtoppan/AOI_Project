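; Actor grouping three boulder Geometry Collection components (big drop, small, hop), apparently for a falling-rock destruction effect.
; On BeginPlay it hides all three collections, without propagating to child components.
; An unconnected branch checks for an "Instrument" actor tag to set a Visible variable and enable physics and gravity on the boulders, but it never runs.
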(event EventBeginPlay
  (Rendering|SetVisibility (Variables|Default|GetboulderDropBig_GeometryCollection) false false))

(fn ConstructionScript)