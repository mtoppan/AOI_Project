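; BP_HornInstrument is a horn instrument actor with events for idle effects, HUD feedback and playing the horn.
; Show and hide events toggle the NSHornIdle effect, while PlayWeakerHornEffects plays a wrong-timing sound and calls WrongBeat on the BP_HUD widget.
; PlayHornSound sets HornTrackOn when AddedTrack is false, then both branches reach a one-second delay.
; Icon, clef and horn-use HUD updates are unfinished casts, and AddHornTrack is empty.
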(event EventBeginPlay)

(event Collision|EventActorBeginOverlap
  (params (OtherActor :type Actor%20Object%20Reference)))

(event EventTick
  (params (DeltaSeconds :type Float%20%28single-precision%29)))

(event EventShowEffects
  (Components|Activation|Activate (Variables|Default|GetNS_HornIdle) false))

(event EventHideEffects
  (Components|Activation|Deactivate (Variables|Default|GetNS_HornIdle)))

(event EventShowMusicClef
  (bind _asbp_hud (Utilities|Casting|CastToBP_HUD (HUD|GetHUD (Game|GetPlayerController 0)))) ; requires ui function for adding horn + clef
)

(event EventPlayWeakerHornEffects
  (Audio|PlaySound2D "/Game/Sounds/SFX/WrongTiming.WrongTiming" 3.0 1.0 0.0 0 0)
  (bind _asbp_hud (Utilities|Casting|CastToBP_HUD (HUD|GetHUD (Game|GetPlayerController 0))))
  (Default|WrongBeat (Variables|/Game/Blueprints/BP_HUD.BP_HUD_C|GetHUDWidget _asbp_hud)))

(event EventPlayHornSound
  (if (Variables|Default|GetAddedTrack)
    (bind _asbp_hud (Utilities|Casting|CastToBP_HUD (HUD|GetHUD (Game|GetPlayerController 0)))) ; ui for using horn
    (else
      (Variables|Default|SetHornTrackOn true)))
  (Utilities|FlowControl|Delay 1.0))

(event EventAddHornTrack)

(event EventShowHornIcon
  (bind _asbp_hud (Utilities|Casting|CastToBP_HUD (HUD|GetHUD (Game|GetPlayerController 0)))) ; ui for picking up horn
)

(fn ConstructionScript)