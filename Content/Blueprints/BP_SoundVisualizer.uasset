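; BP_SoundVisualizer is an actor that makes crystal meshes glow blue in response to analyzed audio loudness.
; On BeginPlay it gets the music manager's cave percussion audio and creates dynamic M_crystal instances for its root's child primitives.
; Each Tick it samples the Analyzer's normalized channel loudness at game time minus a fixed offset.
; The squared loudness blends each crystal's emissive color from black to blue.
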(event EventTick
  (params (DeltaSeconds :type Float%20%28single-precision%29))
  (bind _returnvalue (Utilities|Time|GetGameTimeinSeconds))
  (bind _analyzer (Variables|Default|GetAnalyzer))
  (bind _returnvalue_2 (- _returnvalue 0.160249))
  (bind _outloudness (Class|LoudnessNRT|GetNormalizedChannelLoudnessatTime _analyzer _returnvalue_2 1))
  (for _array_element (Variables|Default|GetMatInstances)
    (bind _asmaterial_instance_dynamic (Utilities|Casting|CastToMaterialInstanceDynamic _array_element))
    (Rendering|Material|SetVectorParameterValue _asmaterial_instance_dynamic "Emissive_Col" (Math|Color|Lerp(LinearColor) "(R=0.000000,G=0.000000,B=0.000000,A=1.000000)" "(R=0.000000,G=0.027410,B=1.000000,A=1.000000)" (* _outloudness _outloudness)) :!class /Script/Engine.MaterialInstanceDynamic)))

(event EventBeginPlay
  (bind _returnvalue (Actor|GetActorOfClass "/Game/Blueprints/BP_MusicManager.BP_MusicManager_C"))
  (Variables|Default|SetAudio (Variables|/Game/Blueprints/BP_MusicManager.BP_MusicManager_C|GetCavePercussion _returnvalue))
  (Variables|Default|SetDuration (Variables|/Script/Engine.SoundBase|GetDuration (Variables|/Script/AudioAnalyzer.AudioAnalyzerNRT|GetSound (Variables|Default|GetAnalyzer))))
  (for _array_element (Components|GetChildrenComponents (Variables|Default|GetDefaultSceneRoot) false)
    (bind _asprimitive_component (Utilities|Casting|CastToPrimitiveComponent _array_element))
    (bind _returnvalue_2 (Rendering|Material|CreateDynamicMaterialInstance _asprimitive_component 0 "/Game/Materials/M_crystal.M_crystal" "None" :!class /Script/Engine.PrimitiveComponent))
    (Utilities|Array|Add (Variables|Default|GetMatInstances) _returnvalue_2)))

(fn ConstructionScript)