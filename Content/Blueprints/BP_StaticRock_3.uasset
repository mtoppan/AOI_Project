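; BP_StaticRock_3 is a rock actor that reacts to a playing percussion instrument overlapping it.
; BeginPlay hides its geometry collection and creates dynamic materials for four slots.
; An overlapping Instrument-tagged PercussionInstrument that is playing triggers a shatter sound and a timeline driving those materials' Alpha, though nothing here re-shows the collection.
; A separate PlayLandSFX event, not called here, plays a bounce sound and a brief Niagara landing burst.
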(event Custom|PlayLandSFX
  (bind _ns_rocklandbig1 (Variables|Default|GetNS_RockLandBig1))
  (Audio|PlaySoundatLocation "/Game/Sounds/SFX/rockBounceLarge.rockBounceLarge" (Transformation|GetWorldLocation (Variables|Default|GetRockBlocks_MedRockBlockA)) "0, 0, 0" 1.0 1.0 0.0 "/Game/Sounds/SFX/SA_Rocks.SA_Rocks" 0 0 0)
  (Components|Activation|Activate _ns_rocklandbig1 false)
  (Utilities|FlowControl|Delay 0.2)
  (Components|Activation|Deactivate _ns_rocklandbig1))

(event Custom|FadeAlpha
  (bind _alphatrack (Timeline|Timeline_0 Play)
    (:Update
      (Rendering|Material|SetScalarParameterValue (stale EventBeginPlay _returnvalue) "Alpha" _alphatrack :!class /Script/Engine.MaterialInstanceDynamic)
      (Rendering|Material|SetScalarParameterValue (stale EventBeginPlay _returnvalue_2) "Alpha" _alphatrack :!class /Script/Engine.MaterialInstanceDynamic)
      (Rendering|Material|SetScalarParameterValue (stale EventBeginPlay _returnvalue_3) "Alpha" _alphatrack :!class /Script/Engine.MaterialInstanceDynamic)
      (Rendering|Material|SetScalarParameterValue (stale EventBeginPlay _returnvalue_4) "Alpha" _alphatrack :!class /Script/Engine.MaterialInstanceDynamic))))

(event Collision|EventActorBeginOverlap
  (params (OtherActor :type Actor%20Object%20Reference))
  (if (Actor|ActorHasTag OtherActor "Instrument")
    (bind _aspercussion_instrument (Utilities|Casting|CastToPercussionInstrument OtherActor))
    (if (Variables|/Script/AOI_Project.PercussionInstrument|GetPlaying _aspercussion_instrument)
      (CallFunction|FadeAlpha)
      (Audio|PlaySound2D "/Game/Sounds/SFX/rockShatterBig.rockShatterBig" 1.4 1.0 0.0 0 0))))

(event EventBeginPlay
  (bind _static_medrockblockb_geometrycollection (Variables|Default|GetStatic_MedRockBlockB_GeometryCollection))
  (Rendering|SetVisibility _static_medrockblockb_geometrycollection false false)
  (bind _returnvalue (Rendering|Material|CreateDynamicMaterialInstance _static_medrockblockb_geometrycollection 0 0 "None" :!class /Script/Engine.PrimitiveComponent))
  (bind _returnvalue_2 (Rendering|Material|CreateDynamicMaterialInstance _static_medrockblockb_geometrycollection 1 0 "None" :!class /Script/Engine.PrimitiveComponent))
  (bind _returnvalue_3 (Rendering|Material|CreateDynamicMaterialInstance _static_medrockblockb_geometrycollection 2 0 "None" :!class /Script/Engine.PrimitiveComponent))
  (bind _returnvalue_4 (Rendering|Material|CreateDynamicMaterialInstance _static_medrockblockb_geometrycollection 3 0 "None" :!class /Script/Engine.PrimitiveComponent)))

(fn ConstructionScript)