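; BP_TrrigerSpaceBarUI is a trigger actor that shows a one-time "E to play" prompt to a player who has the drum.
; On overlap by a Player-tagged actor, it checks GotDrum on BP_Player, calls ShowEToPlay on the BP_HUD widget and sets Introduced.
; End overlap calls HideEToPlay only while Introduced is false, so it does not hide a prompt this trigger has shown.
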(event Collision|EventActorBeginOverlap
  (params (OtherActor :type Actor%20Object%20Reference))
  (if (Actor|ActorHasTag OtherActor "Player")
    (if (not (Variables|Default|GetIntroduced))
      (bind _returnvalue (Actor|GetActorOfClass "/Game/Blueprints/BP_Player.BP_Player_C"))
      (if (Variables|/Script/AOI_Project.BasePlayer|GetGotDrum _returnvalue)
        (bind _asbp_hud (Utilities|Casting|CastToBP_HUD (HUD|GetHUD (Game|GetPlayerController 0))))
        (Default|ShowEtoPlay (Variables|/Game/Blueprints/BP_HUD.BP_HUD_C|GetHUDWidget _asbp_hud))
        (Variables|Default|SetIntroduced true)))))

(event Collision|EventActorEndOverlap
  (params (OtherActor :type Actor%20Object%20Reference))
  (if (Actor|ActorHasTag OtherActor "Player")
    (if (not (Variables|Default|GetIntroduced))
      (bind _asbp_hud (Utilities|Casting|CastToBP_HUD (HUD|GetHUD (Game|GetPlayerController 0))))
      (Default|HideEtoPlay (Variables|/Game/Blueprints/BP_HUD.BP_HUD_C|GetHUDWidget _asbp_hud)))))

(fn ConstructionScript)