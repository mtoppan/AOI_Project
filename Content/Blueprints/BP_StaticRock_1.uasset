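; BP_StaticRock_1 is a rock actor that a playing percussion instrument shatters on overlap.
; BeginPlay hides its geometry collection and creates six dynamic material instances on it.
; An overlap by a playing PercussionInstrument tagged "Instrument" plays a shatter sound, disables Sphere1 collision after a short delay, and drives the materials' Alpha by timeline before destroying the actor.
; A separate PlayLandSFX event plays a bounce sound and briefly activates landing Niagara effects.
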(event Custom|PlayLandSFX
  (Audio|PlaySoundatLocation "/Game/Sounds/SFX/rockBounceLarge.rockBounceLarge" (Transformation|GetWorldLocation (Variables|Default|GetRockBlocks_LargeRockBlockA)) "0, 0, 0" 1.0 1.0 0.0 "/Game/Sounds/SFX/SA_Rocks.SA_Rocks" 0 0 0)
  (Components|Activation|Activate (Variables|Default|GetNS_RockLandBig) false)
  (Utilities|FlowControl|Delay 0.2)
  (Components|Activation|Deactivate (Variables|Default|GetNS_RockLandBig)))

(event Custom|FadeAlpha
  (Utilities|FlowControl|Delay 0.05)
  (Collision|SetCollisionEnabled (Variables|Default|GetSphere1) "NoCollision")
  (bind _alphatrack (Timeline|Timeline_0 Play)
    (:Update
      (Rendering|Material|SetScalarParameterValue (stale EventBeginPlay _returnvalue) "Alpha" _alphatrack :!class /Script/Engine.MaterialInstanceDynamic)
      (Rendering|Material|SetScalarParameterValue (stale EventBeginPlay _returnvalue_2) "Alpha" _alphatrack :!class /Script/Engine.MaterialInstanceDynamic)
      (Rendering|Material|SetScalarParameterValue (stale EventBeginPlay _returnvalue_3) "Alpha" _alphatrack :!class /Script/Engine.MaterialInstanceDynamic)
      (Rendering|Material|SetScalarParameterValue (stale EventBeginPlay _returnvalue_4) "Alpha" _alphatrack :!class /Script/Engine.MaterialInstanceDynamic)
      (Rendering|Material|SetScalarParameterValue (stale EventBeginPlay _returnvalue_5) "Alpha" _alphatrack :!class /Script/Engine.MaterialInstanceDynamic)
      (Rendering|Material|SetScalarParameterValue (stale EventBeginPlay _returnvalue_6) "Alpha" _alphatrack :!class /Script/Engine.MaterialInstanceDynamic))
    (:Finished
      (Actor|DestroyActor))))

(event Collision|EventActorBeginOverlap
  (params (OtherActor :type Actor%20Object%20Reference))
  (if (Actor|ActorHasTag OtherActor "Instrument")
    (bind _aspercussion_instrument (Utilities|Casting|CastToPercussionInstrument OtherActor))
    (if (Variables|/Script/AOI_Project.PercussionInstrument|GetPlaying _aspercussion_instrument)
      (CallFunction|FadeAlpha)
      (Audio|PlaySound2D "/Game/Sounds/SFX/rockShatterBig.rockShatterBig" 1.4 1.0 0.0 0 0))))

(event EventBeginPlay
  (bind _staticbarrier_largerockblocka_geometrycollection (Variables|Default|GetStaticBarrier_LargeRockBlockA_GeometryCollection))
  (Rendering|SetVisibility _staticbarrier_largerockblocka_geometrycollection false false)
  (bind _returnvalue (Rendering|Material|CreateDynamicMaterialInstance _staticbarrier_largerockblocka_geometrycollection 0 0 "None" :!class /Script/Engine.PrimitiveComponent))
  (bind _returnvalue_2 (Rendering|Material|CreateDynamicMaterialInstance _staticbarrier_largerockblocka_geometrycollection 1 0 "None" :!class /Script/Engine.PrimitiveComponent))
  (bind _returnvalue_3 (Rendering|Material|CreateDynamicMaterialInstance _staticbarrier_largerockblocka_geometrycollection 2 0 "None" :!class /Script/Engine.PrimitiveComponent))
  (bind _returnvalue_4 (Rendering|Material|CreateDynamicMaterialInstance _staticbarrier_largerockblocka_geometrycollection 3 0 "None" :!class /Script/Engine.PrimitiveComponent))
  (bind _returnvalue_5 (Rendering|Material|CreateDynamicMaterialInstance _staticbarrier_largerockblocka_geometrycollection 4 0 "None" :!class /Script/Engine.PrimitiveComponent))
  (bind _returnvalue_6 (Rendering|Material|CreateDynamicMaterialInstance _staticbarrier_largerockblocka_geometrycollection 5 0 "None" :!class /Script/Engine.PrimitiveComponent)))

(fn ConstructionScript)