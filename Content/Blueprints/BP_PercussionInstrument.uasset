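; Drum instrument actor that plays hit feedback, shatters rocks and adds the cave percussion layer to the music.
; While playing, overlapping "Rock" actors reveal "Crack"-tagged geometry collections, broken by a radial Chaos strain field, then are destroyed after delays.
; Events drive HUD prompts and icons, idle effects, and the music manager's percussion volume.
; Hits trigger sound, Niagara waves and camera shake, with weaker feedback for wrong timing.
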(event EventPlayDrumSound
  (bind _returnvalue (Game|GetPlayerController 0))
  (bind _returnvalue_2 (HUD|GetHUD _returnvalue))
  (Audio|PlaySoundatLocation "/Game/Sounds/SFX/DrumHit.DrumHit" (Transformation|GetActorLocation) "0, 0, 0" 1.0 1.0 0.0 0 0 0 0)
  (Components|Activation|Activate (Variables|Default|GetNS_DrumSoundWave) false)
  (Components|Activation|Activate (Variables|Default|GetNS_DrumSoundWaveEcho) false)
  (Camera|PlayWorldCameraShake "/Game/Blueprints/BP_CameraShake.BP_CameraShake_C" (Transformation|GetActorLocation) 0.0 5e+02)
  (if (Variables|Default|GetAddedTrack)
    (bind _asbp_hud (Utilities|Casting|CastToBP_HUD _returnvalue_2))
    (Default|UseDrum (Variables|/Game/Blueprints/BP_HUD.BP_HUD_C|GetHUDWidget _asbp_hud))
    (else
      (bind _asbp_hud_2 (Utilities|Casting|CastToBP_HUD _returnvalue_2))))
  (Default|HideEtoPlay (Variables|/Game/Blueprints/BP_HUD.BP_HUD_C|GetHUDWidget _asbp_hud_2))
  (Variables|Default|SetDrumTrackOn true)
  (Utilities|FlowControl|Delay 1.0)
  (Components|Activation|Deactivate (Variables|Default|GetNS_DrumSoundWave))
  (Components|Activation|Deactivate (Variables|Default|GetNS_DrumSoundWaveEcho)))

(event Collision|EventActorBeginOverlap
  (params (OtherActor :type Actor%20Object%20Reference))
  (if (Actor|ActorHasTag OtherActor "Rock")
    (if (Variables|Default|GetPlaying)
      (for _array_element (Actor|GetComponentsbyTag OtherActor "/Script/GeometryCollectionEngine.GeometryCollectionComponent" "Crack")
        (Rendering|SetVisibility _array_element true false)
        (Physics|SetSimulatePhysics _array_element true)
        (Class|FieldSystemComponent|ApplyPhysicsField (Variables|Default|GetFieldSystem1) true "Field_ExternalClusterStrain" 0 (Field|SetRadialFalloff (Variables|Default|GetRadialFalloff) (Variables|Default|GetInstrument%20Force) 0.0 1.0 0.0 (Components|Sphere|GetScaledSphereRadius (Variables|Default|GetSphereCollision)) (Transformation|GetActorLocation OtherActor) "Field_FallOff_None"))
        (for _array_element_2 (Actor|GetComponentsbyTag OtherActor "/Script/Engine.SkeletalMeshComponent" "Crack")
          (Rendering|SetVisibility _array_element_2 false false)
          (Utilities|FlowControl|Delay 0.05)
          (for _array_element_3 (Actor|GetComponentsbyTag OtherActor "/Script/Engine.SphereComponent" "Crack")
            (Collision|SetCollisionEnabled _array_element_3 "NoCollision")
            (Utilities|FlowControl|Delay 2.0)
            (Actor|DestroyActor OtherActor)))))))

(event EventShowDrumIcon
  (Default|PickupDrum (Variables|/Game/Blueprints/BP_HUD.BP_HUD_C|GetHUDWidget (stale EventShowUI _asbp_hud))))

(event EventAddDrumTrack
  (bind _returnvalue (Actor|GetActorOfClass "/Game/Blueprints/BP_MusicManager.BP_MusicManager_C"))
  (Audio|Components|Audio|AdjustVolume (Variables|/Game/Blueprints/BP_MusicManager.BP_MusicManager_C|GetCavePercussion _returnvalue) 0.0 1.0 "Linear" :!class /Script/Engine.AudioComponent))

(event EventShowUI
  (bind _asbp_hud (Utilities|Casting|CastToBP_HUD (HUD|GetHUD (Game|GetPlayerController 0))))
  (Default|HideE (Variables|/Game/Blueprints/BP_HUD.BP_HUD_C|GetHUDWidget _asbp_hud))
  (Default|ShowEtoPlay (Variables|/Game/Blueprints/BP_HUD.BP_HUD_C|GetHUDWidget _asbp_hud)))

(event EventPlayWeakerDrumEffects
  (Camera|PlayWorldCameraShake "/Game/Blueprints/BP_WeakCameraShake.BP_WeakCameraShake_C" (Transformation|GetActorLocation) 0.0 5e+02)
  (Components|Activation|Activate (Variables|Default|GetNS_WeakDrum) false)
  (Audio|PlaySound2D "/Game/Sounds/SFX/WrongTiming.WrongTiming" 3.0 1.0 0.0 0 0)
  (Components|Activation|Deactivate (Variables|Default|GetNS_WeakDrum))
  (bind _asbp_hud (Utilities|Casting|CastToBP_HUD (HUD|GetHUD (Game|GetPlayerController 0))))
  (Default|WrongBeat (Variables|/Game/Blueprints/BP_HUD.BP_HUD_C|GetHUDWidget _asbp_hud)))

(event EventShowMusicClef
  (bind _asbp_hud (Utilities|Casting|CastToBP_HUD (HUD|GetHUD (Game|GetPlayerController 0))))
  (Default|UseDrumandAddTrack (Variables|/Game/Blueprints/BP_HUD.BP_HUD_C|GetHUDWidget _asbp_hud)))

(event EventShowEffects
  (Rendering|SetVisibility (Variables|Default|GetPointLight) true false)
  (Components|Activation|SetActive (Variables|Default|GetNS_DrumIdle) true false))

(event EventHideEffects
  (Rendering|SetVisibility (Variables|Default|GetPointLight) false false)
  (Components|Activation|SetActive (Variables|Default|GetNS_DrumIdle) false false))

(fn ConstructionScript)