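; BP_Ball is a rhythmic bouncing ball whose Rock component moves and squashes along a timeline.
; BeginPlay scales the timeline's play rate from BPM, as 100 divided by BPM.
; Timeline tracks drive vertical and sideways (Y-axis) offsets plus squash scale, and a Hit Ground event spawns an emitter at the rock.
; No exec wire starts the timeline in the graph, and the emitter call shows no template.
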(event EventBeginPlay
  (Components|Timeline|SetPlayRate (Variables|Default|GetTimeline_Rock) (/ 1e+02 (Variables|Default|GetBPM))))

(fn ConstructionScript)